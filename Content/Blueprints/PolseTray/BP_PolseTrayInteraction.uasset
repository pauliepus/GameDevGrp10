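; BP_PolseTrayInteraction is a tray that keeps a Points count of cooked Poels actors placed on it.
; Overlap begin adds a point for a cooked Poels.
; Overlap end waits briefly, then subtracts one only if the cooked actor is still valid and the wave manager's ManagerStartWaveEnded flag is false, so destroyed actors keep their point.
; The wave manager is the first BP_WaveManager found at BeginPlay, when Points also resets.
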(event `self.ReceiveBeginPlay`
  ;[1 1 1] Pregame
  (set `self.Points` 0)
  (bind _outactors (`GameplayStatics.GetAllActorsOfClass` "/Game/Blueprints/Enemies/BP_WaveManager.BP_WaveManager_C"))
  (set `self.WaveReferencePoints` (`|GetArrayItem` _outactors)))

(event `self.ReceiveActorBeginOverlap`
  (params (OtherActor :type "Actor Object Reference"))
  ;[1 1 1] Points
  (bind _aspoels (cast `Poels` OtherActor))
  (if (`Poels.bIsCooked` _aspoels)
    (set `self.Points` (+ (`self.Points`) 1))))

(event `self.ReceiveActorEndOverlap`
  (params (OtherActor :type "Actor Object Reference"))
  ;[1 1 1] Points
  (`KismetSystemLibrary.Delay` 0.2)
  (if (`WaveManager.ManagerStartWaveEnded` (`self.WaveReferencePoints`))
    _
    (elif (`KismetSystemLibrary.IsValid` OtherActor)
      (bind _aspoels (cast `Poels` OtherActor))
      (if (`Poels.bIsCooked` _aspoels)
        (if true
          (set `self.Points` (- (`self.Points`) 1)))))))

(fn `UserConstructionScript`)