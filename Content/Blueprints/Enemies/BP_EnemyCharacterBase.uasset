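; Base enemy character that moves toward a destination, steals on arrival and dies when shot.
; On BeginPlay it runs AI MoveTo toward the DEMO target, calling EnemySteal on success and retrying after a short delay on failure.
; Overlapping a BP_Bullet calls EnemyDie; neither that nor EnemySteal has logic in this graph.
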(event `self.ReceiveBeginPlay`
  ;[1 1 1] Movement
  (`self.EnemyMove`))

(event `EnemyMove`
  ;[1 1 1] Movement
  (`|AIMoveTo` self (`self.[DEMO]`) null 100.0
    (:`OnSuccess`
      (`self.EnemySteal`))
    (:`OnFail`
      (`KismetSystemLibrary.Delay` 0.2)
      (`self.EnemyMove`))))

(event `self.ReceiveActorBeginOverlap`
  (params (OtherActor :type "Actor Object Reference"))
  ;[1 1 1] Bullet overlap = Death
  (cast `/Game/Blueprints/Actors/BP_Bullet` OtherActor)
  (`self.EnemyDie`))

(fn `UserConstructionScript`)