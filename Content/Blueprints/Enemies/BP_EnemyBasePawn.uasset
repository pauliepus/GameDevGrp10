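; BP_EnemyBasePawn is a base enemy pawn that wanders at random, starting on BeginPlay.
; The MoveEnemy event picks a random reachable navmesh point near the pawn's current location and issues an AI MoveTo toward it.
; It re-calls itself after a delay, longer on success and shorter on failure, forming an endless roam loop.
; Each move request also prints a placeholder debug string.
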(event `self.ReceiveBeginPlay`
  (`self.MoveEnemy`))

(event `MoveEnemy`
  ;[1 1 1] Movement based on PK Easter guide
  (bind _output_get (set `self.Random Location` (`NavigationSystemV1.K2_GetRandomReachablePointInRadius` (`self.K2_GetActorLocation`) 300.0 null null)))
  (`|AIMoveTo` self _output_get null
    (:`then`
      (`KismetSystemLibrary.PrintString` "Hello"))
    (:`OnSuccess`
      (`KismetSystemLibrary.Delay` 4.0)
      (`self.MoveEnemy`))
    (:`OnFail`
      (`KismetSystemLibrary.Delay` 1.0)
      (`self.MoveEnemy`))))

(fn `UserConstructionScript`)