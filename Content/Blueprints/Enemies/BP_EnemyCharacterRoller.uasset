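; Enemy character that repeatedly charges the player from its spawn point and can steal a Pølse.
; A recursive AIMoveTo loop approaches crouched until half the distance remains, then plays a rolling animation, uncrouches, closes in and returns to base.
; A failed first approach retries after a short delay.
; Bullet overlap triggers EnemyDie, while hitting a Pølse destroys both it and the roller with a squeal.
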(event `self.ReceiveBeginPlay`
  ;[1 1 1] Movement
  (set `self.RollerBaseLocation` (`self.K2_GetActorLocation` self))
  (`self.EnemyMove`))

(event `self.EnemyMove`
  (bind _returnvalue (`self.K2_GetActorLocation` (`GameplayStatics.GetPlayerPawn` 0)))
  ;[1 1 1] Movement
  (`GameplayStatics.PlaySoundAtLocation` "/Game/Sound/Sound_Effects/Enemy/SilenceOther_Sounds_-_Mythical_Creatures_-_Small_Critter_Running_.SilenceOther_Sounds_-_Mythical_Creatures_-_Small_Critter_Running_" (`self.RollerBaseLocation`) (struct) 1.0 1.0 0.0 null null null null)
  (`self.Crouch`)
  (`|AIMoveTo` self _returnvalue null (/ (`KismetMathLibrary.Distance2D` (`KismetMathLibrary.Conv_VectorToVector2D` _returnvalue) (`KismetMathLibrary.Conv_VectorToVector2D` (`self.K2_GetActorLocation`))) 2.0)
    (:`OnSuccess`
      (`SkeletalMeshComponent.PlayAnimation` (`self.Mesh`) "/Game/Characters/Creature_Enemies/EnemyCreatureRoll_Creature_Armature_Roll.EnemyCreatureRoll_Creature_Armature_Roll" true)
      (`self.UnCrouch`)
      (`|AIMoveTo` self (`self.K2_GetActorLocation` (`GameplayStatics.GetPlayerPawn` 0)) null 100.0
        (:`OnSuccess`
          _)
        (:`OnFail`
          _))
      (`|AIMoveTo` self (`self.RollerBaseLocation`) null
        (:`OnSuccess`
          _)
        (:`OnFail`
          _))
      (`self.EnemyMove`))
    (:`OnFail`
      (`KismetSystemLibrary.Delay` 0.2)
      (`self.EnemyMove`))))

(event `self.ReceiveActorBeginOverlap`
  (params (OtherActor :type "Actor Object Reference"))
  ;[1 1 1] Bullet overlap = Death, Pølse overlap = Steal
  (cast `/Game/Blueprints/Actors/BP_Bullet` OtherActor)
  (`self.EnemyDie`))

(event `self.ReceiveHit`
  (params (MyComp :type "PrimitiveComponent Object Reference") (Other :type "Actor Object Reference") (OtherComp :type "PrimitiveComponent Object Reference") (bSelfMoved :type Boolean) (HitLocation :type "Vector Structure") (HitNormal :type "Vector Structure") (NormalImpulse :type "Vector Structure") (Hit :type "HitResult Structure (by ref)"))
  ;[1 1 1] Bullet overlap = Death, Pølse overlap = Steal
  (bind _asbp_poelse (cast `/Game/Blueprints/Poels/BP_Poelse` Other))
  (`self.K2_DestroyActor` _asbp_poelse)
  (`GameplayStatics.PlaySoundAtLocation` "/Game/Sound/Sound_Effects/Enemy/Gamemaster_Audio_-_Creature_Voices__-_Toyish_Squeal_Playful_Happy.Gamemaster_Audio_-_Creature_Voices__-_Toyish_Squeal_Playful_Happy" (`self.K2_GetActorLocation` self) (struct) 1.0 1.0 0.0 null null null null)
  (`self.K2_DestroyActor`))

(fn `UserConstructionScript`
  (`parent.UserConstructionScript`))