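; BP_Poelse is a sausage actor that shows whether it is uncooked, cooked or burnt.
; Every Tick it reads IsCooked and IsOvercooked and sets the matching material on SKDefault, with IsCooked taking priority; this graph never sets either flag.
; BeginPlay only binds PhysicalAnimation to the skeletal mesh.
; The nodes meant to make it floppy through physics are unconnected and never run.
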(event `self.ReceiveTick`
  (params (DeltaSeconds :type "Float (single-precision)"))
  (bind _skdefault (`self.SKDefault`))
  ;[0.07 0 0.001438] Per tick Check Material
  ;;[0.9036 0.97 0] The bools it checks
  (if (`self.IsCooked`)
    (`PrimitiveComponent.SetMaterial` _skdefault 0 "/Game/Assets/Finals/CampingGear/Materials/M_Polse_Cooked.M_Polse_Cooked")
    (elif (`self.IsOvercooked`)
      (`PrimitiveComponent.SetMaterial` _skdefault 0 "/Game/Assets/Finals/CampingGear/Materials/M_Polse_Burnt.M_Polse_Burnt")
      (else
        (`PrimitiveComponent.SetMaterial` _skdefault 0 "/Game/Assets/Finals/CampingGear/Materials/M_Polse_Uncooked.M_Polse_Uncooked")))))

(event `self.ReceiveBeginPlay`
  ;[0.59 0.1212 0] Should make object floppy
  (`PhysicalAnimationComponent.SetSkeletalMeshComponent` (`self.PhysicalAnimation`) (`self.SKDefault`)))

(fn `UserConstructionScript`)