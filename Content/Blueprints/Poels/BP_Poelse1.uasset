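; BP_Poelse1 is a sausage actor that becomes cooked as soon as it begins overlapping a GrillActor.
; Tick reapplies the uncooked, cooked or burnt material from IsCooked and IsOvercooked, with cooked taking priority; nothing in this graph sets overcooked.
; BeginPlay binds PhysicalAnimation to the skeletal mesh for a floppy body, but the physics simulation setup is left unconnected.
; Ending the grill overlap only casts and has no effect.
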(event `self.ReceiveActorBeginOverlap`
  (params (OtherActor :type "Actor Object Reference"))
  (cast `GrillActor` OtherActor)
  (`self.SetIsCookedTrue`))

(event `self.ReceiveActorEndOverlap`
  (params (OtherActor :type "Actor Object Reference"))
  (cast `GrillActor` OtherActor))

(event `self.ReceiveBeginPlay`
  ;[0.59 0.1212 0] Should make object floppy
  (`PhysicalAnimationComponent.SetSkeletalMeshComponent` (`self.PhysicalAnimation`) (`self.SKDefault`)))

(event `self.ReceiveTick`
  (params (DeltaSeconds :type "Float (single-precision)"))
  (bind _skdefault (`self.SKDefault`))
  ;[0.07 0 0.001438] Per tick Check Material
  ;;[0.9036 0.97 0] The bools it checks
  (if (`self.bIsCooked`)
    (`PrimitiveComponent.SetMaterial` _skdefault 0 "/Game/Assets/Finals/CampingGear/Materials/M_Polse_Cooked.M_Polse_Cooked")
    (elif (`self.bIsOvercooked`)
      (`PrimitiveComponent.SetMaterial` _skdefault 0 "/Game/Assets/Finals/CampingGear/Materials/M_Polse_Burnt.M_Polse_Burnt")
      (else
        (`PrimitiveComponent.SetMaterial` _skdefault 0 "/Game/Assets/Finals/CampingGear/Materials/M_Polse_Uncooked.M_Polse_Uncooked")))))

(fn `UserConstructionScript`)