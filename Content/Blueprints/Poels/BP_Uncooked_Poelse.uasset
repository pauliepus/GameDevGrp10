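; BP_Uncooked_Poelse is an uncooked sausage actor that starts cooking when it overlaps a GrillActor.
; BeginPlay caches the first BP_WaveManager and binds the skeletal mesh to a PhysicalAnimation component.
; Grill overlap calls SetIsCookedTrue, rechecking every five seconds while the wave has ended; leaving calls StopTimers.
; The physics asset, physical animation settings and body simulation nodes for floppiness are disconnected, so never run.
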(event `self.ReceiveBeginPlay`
  ;[1 1 1] Getting waveManager reference
  (bind _outactors (`GameplayStatics.GetAllActorsOfClass` "/Game/Blueprints/Enemies/BP_WaveManager.BP_WaveManager_C"))
  (set `self.WaveManagerReference` (`|GetArrayItem` _outactors))
  ;[0.59 0.1212 0] Should make object floppy
  (`PhysicalAnimationComponent.SetSkeletalMeshComponent` (`self.PhysicalAnimation`) (`self.SKDefault`)))

(event `self.ReceiveActorBeginOverlap`
  (params (OtherActor :type "Actor Object Reference"))
  (if (`WaveManager.ManagerWaveEnded` (`self.WaveManagerReference`)) :!label _label
    (`KismetSystemLibrary.Delay` 5.0)
    (goto _label)
    (else
      (cast `GrillActor` OtherActor)
      (`self.SetIsCookedTrue`))))

(event `self.ReceiveActorEndOverlap`
  (params (OtherActor :type "Actor Object Reference"))
  (cast `GrillActor` OtherActor)
  (`self.StopTimers`))

(fn `UserConstructionScript`)