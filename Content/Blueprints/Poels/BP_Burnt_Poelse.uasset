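; BP_Burnt_Poelse is the burnt variant of a pølse (sausage) actor.
; On BeginPlay it caches the level's first BP_WaveManager, flags itself as cooked and binds its PhysicalAnimation component to the SKDefault skeletal mesh.
; The nodes meant to make it floppy through physics asset, physical animation settings and body simulation are left unwired and never run.
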(event `self.ReceiveBeginPlay`
  ;[1 1 1] Getting waveManager reference
  (bind _outactors (`GameplayStatics.GetAllActorsOfClass` "/Game/Blueprints/Enemies/BP_WaveManager.BP_WaveManager_C"))
  (set `self.WaveManagerReference` (`|GetArrayItem` _outactors))
  (set `self.bIsCooked` true) ; Burnt Poels
  ;[0.59 0.1212 0] Should make object floppy
  (`PhysicalAnimationComponent.SetSkeletalMeshComponent` (`self.PhysicalAnimation`) (`self.SKDefault`)))

(fn `UserConstructionScript`)