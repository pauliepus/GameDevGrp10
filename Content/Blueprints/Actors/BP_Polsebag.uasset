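; BP_Polsebag is an interactable actor with placeholder interaction logic.
; OnInteraction only prints a debug string.
; LineTraceInteractFromPlayer runs a Visibility trace from the player's MeshFPV, ignoring the player, and leaves the result unused.
; The trace offset multiplies the forward vector component-wise by an X-only vector, so it extends only along world X rather than following the full view direction.
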(event `/Game/Blueprints/BPI_Interaction.On Interaction`
  (params (InteractButton :type Boolean))
  (`KismetSystemLibrary.PrintString` "I interact"))

(event `LineTraceInteractFromPlayer`
  (bind _meshfpv (`PlayerCharacter.MeshFPV` (`self.PlayerCharacterReference`)))
  (bind _returnvalue (`SceneComponent.K2_GetComponentLocation` _meshfpv))
  (`KismetSystemLibrary.LineTraceSingle` _returnvalue (+ _returnvalue (* (`SceneComponent.GetForwardVector` _meshfpv) (500.0 0.0 0.0))) "TraceTypeQuery1" false (`|MakeArray` (`self.PlayerCharacterReference`) :!type "Actor Object Reference")))

(fn `UserConstructionScript`)