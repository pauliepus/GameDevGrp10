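; BP_Bullet is a projectile actor that flies in a straight line and destroys itself five seconds after spawning.
; Tick moves it along its Direction variable, scaled by Speed and delta time, using a non-swept SetActorLocation.
; The overlap event is empty, and the logic to spawn a Niagara fire effect on the other actor and destroy the bullet is disconnected, so hits have no effect.
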(event `self.ReceiveBeginPlay`
  (`KismetSystemLibrary.Delay` 5.0)
  (`self.K2_DestroyActor`))

(event `self.ReceiveActorBeginOverlap`
  (params (OtherActor :type "Actor Object Reference")))

(event `self.ReceiveTick`
  (params (DeltaSeconds :type "Float (single-precision)"))
  (`self.K2_SetActorLocation` (+ (`self.K2_GetActorLocation`) (* (`self.Direction`) DeltaSeconds (`self.Speed`)))))

(fn `UserConstructionScript`)