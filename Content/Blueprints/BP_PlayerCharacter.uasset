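; Player character that grabs and carries BP_Poelse and BP_Shotgun actors, and fires a held shotgun.
; Left mouse line-traces from the camera and disables physics on the hit item, which follows HoldingSpot each Tick until release.
; W and S slide HoldingSpot along its local X axis, while Space spawns BP_Bullet aimed along the camera forward when holding the shotgun.
; Also creates the WB_UI widget on BeginPlay and toggles the pause menu.
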(event `Key|SpaceBar`
  (params (Key :type "Key Structure"))
  (bind _returnvalue (`KismetMathLibrary.GetForwardVector` (`SceneComponent.K2_GetComponentRotation` (`self.PlayerCamera`))))
  (:`Pressed`
    (if (`self.CanShoot`)
      (bind _asbp_shotgun (cast `/Game/Blueprints/Pickups/BP_Shotgun` (`self.GrabbedObject`)))
      (bind _returnvalue_2 (`|SpawnActorFromClass` "/Game/Blueprints/Actors/BP_Bullet.BP_Bullet_C" (`KismetMathLibrary.MakeTransform` (`SceneComponent.K2_GetComponentLocation` (`/Game/Blueprints/Pickups/BP_Shotgun.BulletSpawnLocation` _asbp_shotgun)) (`KismetMathLibrary.Conv_VectorToRotator` _returnvalue)) "Undefined" "MultiplyWithRoot" null null))
      (set `/Game/Blueprints/Actors/BP_Bullet.Direction` _returnvalue _returnvalue_2))))

(event `Key|LeftMouseButton`
  (params (Key :type "Key Structure"))
  (bind _returnvalue (`SceneComponent.K2_GetComponentLocation` (`self.PlayerCamera`)))
  ;[1 1 1] Input
  (:`Pressed`
    ;[1 1 1] Sets Active bool
    (bind (_outhit _returnvalue_2) (`KismetSystemLibrary.LineTraceSingle` :`Start` _returnvalue :`End` (+ _returnvalue (* (`KismetMathLibrary.GetForwardVector` (`SceneComponent.K2_GetComponentRotation` (`self.PlayerCamera`))) (500.0 600.0 600.0))) :`TraceChannel` "TraceTypeQuery2" :`DrawDebugType` "ForDuration"))
    (if _returnvalue_2
      (bind _asbp_poelse (cast `/Game/Blueprints/Poels/BP_Poelse` (`.HitActor` (`GameplayStatics.BreakHitResult` _outhit)))
        (:`then`
          (set `self.GrabbedObject` _asbp_poelse))
        (:`CastFailed`
          (bind _asbp_shotgun (cast `/Game/Blueprints/Pickups/BP_Shotgun` (`.HitActor` (`GameplayStatics.BreakHitResult` _outhit))))
          (set `self.GrabbedObject` _asbp_shotgun)
          (set `self.CanShoot` true)))
      (`PrimitiveComponent.SetSimulatePhysics` (`self.GetComponentByClass` (`self.GrabbedObject`) "/Script/Engine.BoxComponent") false)
      (set `self.IsGrabbingObject` true)))
  (:`Released`
    ;[1 1 1] Release the item
    (if (`self.IsGrabbingObject`)
      (set `self.IsGrabbingObject` false)
      (if (`KismetSystemLibrary.IsValid` (`self.GrabbedObject`))
        (`PrimitiveComponent.SetSimulatePhysics` (`self.GetComponentByClass` (`self.GrabbedObject`) "/Script/Engine.BoxComponent") true)
        (set `self.GrabbedObject` null)
        (set `self.CanShoot` false)))))

(event `Key|S`
  (params (Key :type "Key Structure"))
  ;[1 0.2294 0.3493] Moving Object (WS Input)
  ;;[0.9241 1 0.2956] Forward Movement Input
  (:`Pressed`
    (set `self.IsSHeld` true))
  (:`Released`
    (set `self.IsSHeld` false)))

(event `Key|W`
  (params (Key :type "Key Structure"))
  ;[1 0.2294 0.3493] Moving Object (WS Input)
  ;;[0.9241 1 0.2956] BackwardMovementInput
  (:`Pressed`
    (set `self.IsWHeld` true))
  (:`Released`
    (set `self.IsWHeld` false)))

(event `/Game/Blueprints/BPI_Interaction.On Interaction`
  (params (InteractButton :type Boolean))
  ;[0.3748 0.3747 1] location of moving thing
)

(event `self.ReceiveTick`
  (params (DeltaSeconds :type "Float (single-precision)"))
  (bind _iswheld (`self.IsWHeld`))
  (bind _grabbedobject (`self.GrabbedObject`))
  ;[0.3748 0.3747 1] location of moving thing
  ;;[1 0.2294 0.3493] Moving Object (WS Input)
  ;;;[0.3228 1 0.31] Activates Input
  (if (or (`self.IsSHeld`) _iswheld)
    (if _iswheld
      (bind _output_get (set `self.Offset` (1.0 0.0 0.0)))
      (else
        (set `self.Offset` (-1.0 0.0 0.0))))
    (`SceneComponent.K2_AddLocalOffset` (`self.HoldingSpot`) _output_get false false))
  (if (`self.IsGrabbingObject`)
    ;;[1 0.2344 0.2344] Sets where thing is putting object
    (if (`KismetSystemLibrary.IsValid` _grabbedobject)
      (`self.K2_SetActorLocation` _grabbedobject (+ (`SceneComponent.K2_GetComponentLocation` (`self.HoldingSpot`)) (`self.Offset`)) false false))))

(event `self.ReceiveBeginPlay`
  ;[0.9022 0 1] UI
  (bind _returnvalue (`|CreateWidget` "/Game/Widget_Blueprints/WB_UI.WB_UI_C"))
  (`UserWidget.AddToPlayerScreen` _returnvalue 0))

(event `EnhancedInput|/Game/Characters/Player_Character/InputSystems/IA_Pause`
  (params (ActionValue :type Boolean) (ElapsedSeconds :type "Float (double-precision)") (TriggeredSeconds :type "Float (double-precision)") (InputAction :type "InputAction Object Reference" :default "/Game/Characters/Player_Character/InputSystems/IA_Pause.IA_Pause"))
  (bind _returnvalue (`GameplayStatics.GetPlayerController` 0))
  ;[1 1 1] Pause logic
  (:`Triggered`
    (if (`GameplayStatics.IsGamePaused`)
      (`Widget.RemoveFromParent` (stale _returnvalue_2))
      (`GameplayStatics.SetGamePaused` false)
      (`WidgetBlueprintLibrary.SetInputMode_GameOnly` _returnvalue)
      (set `PlayerController.bShowMouseCursor` false _returnvalue)
      (else
        (bind _returnvalue_2 (`|CreateWidget` "/Game/Widget_Blueprints/PauseMenu.PauseMenu_C"))
        (`UserWidget.AddToViewport` _returnvalue_2 0)
        (`GameplayStatics.SetGamePaused` true)
        (`WidgetBlueprintLibrary.SetInputMode_GameAndUIEx` _returnvalue null)
        (set `PlayerController.bShowMouseCursor` true _returnvalue)))))

(fn `UserConstructionScript`)